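; BPC_CheatManage provides debug cheat functions for reading and changing character friendship levels.
; GetRelationships and UpdateRelationships each pass three characters to the matching GameInstance relationship message, with the update also sending a value.
; Each function prints a formatted line per character, reusing the single returned value as the friendship level for all three.
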(fn `GetRelationships`
  (params (`Character 1` :type Name) (`Character 2` :type Name) (`Character 3` :type Name))
  (bind _relationships (message `/Game/Relationships/BPI_Interfaces.GetRelationships` (`GameplayStatics.GetGameInstance`) `Character 1` `Character 2` `Character 3`))
  (`KismetSystemLibrary.PrintText` (`|FormatText` "{Character 1} is at Friendship Level {Value}" `Character 1` _relationships))
  (`KismetSystemLibrary.PrintText` (`|FormatText` "{Character 2} is at Friendship Level {Value}" `Character 2` _relationships))
  (`KismetSystemLibrary.PrintText` (`|FormatText` "{Character 3} is at Friendship Level {Value}" `Character 3` _relationships)))

(fn `UpdateRelationships`
  (params (`Character 1` :type Name) (`Character 2` :type Name) (`Character 3` :type Name) (Value :type Integer))
  (bind _newrelationships (message `/Game/Relationships/BPI_Interfaces.UpdateRelationships` (`GameplayStatics.GetGameInstance`) `Character 1` `Character 2` `Character 3` Value "None"))
  (`KismetSystemLibrary.PrintText` (`|FormatText` "{Character 1} is NOW at Friendship Level {Value}" `Character 1` _newrelationships))
  (`KismetSystemLibrary.PrintText` (`|FormatText` "{Character 2} is NOW at Friendship Level {Value}" `Character 2` _newrelationships))
  (`KismetSystemLibrary.PrintText` (`|FormatText` " {Character 3} is NOW at Friendship Level {Value}" `Character 3` _newrelationships)))